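; Test destructible prop that loses health when damaged and explodes like a barrel when health runs out.
; AnyDamage subtracts damage from Health, then at zero or below spawns a pooled Niagara explosion at the Cylinder's location and destroys the actor.
; Debug prints show health before each hit, the actor's lifespan while it survives, and a message on destruction.
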(event `self.ReceiveAnyDamage`
  (params (Damage :type "Float (single-precision)") (DamageType :type "DamageType Object Reference") (InstigatedBy :type "Controller Object Reference") (DamageCauser :type "Actor Object Reference"))
  (`KismetSystemLibrary.PrintString` (`KismetStringLibrary.Conv_DoubleToString` (`self.Health`)) true true (struct :`R` 1.0 :`B` 0.700586 :`A` 1.0))
  (set `self.Health` (- (`self.Health`) Damage))
  (if (<= (`self.Health`) 0.0)
    (`NiagaraFunctionLibrary.SpawnSystemAtLocation` "/Game/Blueprints/FX/NS_BarrelExplosion.NS_BarrelExplosion" (`SceneComponent.K2_GetComponentLocation` (`self.Cylinder`)) (struct) (1.0 1.0 1.0) false true "AutoRelease")
    (`self.K2_DestroyActor`)
    (`KismetSystemLibrary.PrintString` "Destroyed")
    (else
      (`KismetSystemLibrary.PrintString` (`KismetStringLibrary.Conv_DoubleToString` (`self.GetLifeSpan`))))))

(fn `UserConstructionScript`)