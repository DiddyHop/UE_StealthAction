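; Elevator trigger actor that steps through streamed levels, finding the ElevatorDoor and loading a first test level on BeginPlay.
; Box overlap shifts the door along X, starts loading the next Levels entry, unloads the current one, increments CurrentLevel, then shifts the door back.
; Ending the overlap shifts the door again.
; Fixed delays pace the sequence without waiting for loading, and the StartOpen branch is empty.
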(event `self.ReceiveBeginPlay`
  (`|ExecutionSequence`
    (:`then_0`
      (bind _returnvalue (`GameplayStatics.GetActorOfClass` "/Game/Blueprints/ElevatorDoor.ElevatorDoor_C"))
      (set `self.Elevator Door Ref` _returnvalue)
      (`GameplayStatics.LoadStreamLevelBySoftObjectPtr` "/Game/testMaps/testMapLoading_Level1.testMapLoading_Level1" true))
    (:`then_1`
      (if (`self.StartOpen`)
        _))))

(event `self.Box.OnComponentBeginOverlap`
  (params (OverlappedComponent :type "PrimitiveComponent Object Reference") (OtherActor :type "Actor Object Reference") (OtherComp :type "PrimitiveComponent Object Reference") (OtherBodyIndex :type Integer) (bFromSweep :type Boolean) (SweepResult :type "HitResult Structure (by ref)"))
  (bind _elevator_door_ref (`self.Elevator Door Ref`))
  (bind _returnvalue (`SceneComponent.K2_GetComponentLocation` (`/Game/Blueprints/ElevatorDoor.StaticMesh` (`self.Elevator Door Ref`))))
  (`KismetSystemLibrary.Delay` 0.4)
  (`self.K2_SetActorLocation` _elevator_door_ref (- _returnvalue (250.0 0.0 0.0)) false false)
  (`GameplayStatics.LoadStreamLevelBySoftObjectPtr` (`|GetArrayItem` (`self.Levels`) (+ (`self.CurrentLevel`) 1)) true)
  (`KismetSystemLibrary.Delay` 0.2)
  (`GameplayStatics.UnloadStreamLevelBySoftObjectPtr` (`|GetArrayItem` (`self.Levels`) (`self.CurrentLevel`)))
  (set `self.CurrentLevel` (+ (`self.CurrentLevel`) 1))
  (`KismetSystemLibrary.Delay` 0.4)
  (`self.K2_SetActorLocation` _elevator_door_ref (+ _returnvalue (250.0 0.0 0.0)) false false))

(event `self.Box.OnComponentEndOverlap`
  (params (OverlappedComponent :type "PrimitiveComponent Object Reference") (OtherActor :type "Actor Object Reference") (OtherComp :type "PrimitiveComponent Object Reference") (OtherBodyIndex :type Integer))
  (`KismetSystemLibrary.Delay` 0.4)
  (`self.K2_SetActorLocation` (`self.Elevator Door Ref`) (- (`SceneComponent.K2_GetComponentLocation` (`/Game/Blueprints/ElevatorDoor.StaticMesh` (`self.Elevator Door Ref`))) (250.0 0.0 0.0)) false false))

(fn `UserConstructionScript`)