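; BP_TutMessager is a placeable tutorial messenger that shows text when the player is nearby.
; Every Tick, it compares the first player pawn's distance from the actor against MessageRange, setting its TextRender to MyTutMessage within range and to empty text beyond it.
; The distance comes from GetPointDistanceToLine with a zero direction, which acts as a point-to-point check.
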(event `self.ReceiveTick`
  (params (DeltaSeconds :type "Float (single-precision)"))
  (if (> (`KismetMathLibrary.GetPointDistanceToLine` (`self.K2_GetActorLocation` (`GameplayStatics.GetPlayerPawn` 0)) (`self.K2_GetActorLocation`)) (`self.messageRange`))
    (`TextRenderComponent.K2_SetText` (`self.TextRender`) (`KismetTextLibrary.Conv_StringToText` ""))
    (else
      (`TextRenderComponent.K2_SetText` (`self.TextRender`) (`KismetTextLibrary.Conv_StringToText` (`self.myTutMessage`))))))

(fn `UserConstructionScript`)