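; Trigger actor that opens the level's elevator door once when something overlaps its Box.
; On BeginPlay it caches an ElevatorDoor found with GetActorOfClass, so it needs no manual reference.
; The overlap moves that actor instantly to its StaticMesh's world location plus a fixed X offset, then clears the Valid flag to block repeat triggers.
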(event `self.ReceiveBeginPlay`
  (bind _returnvalue (`GameplayStatics.GetActorOfClass` "/Game/Blueprints/ElevatorDoor.ElevatorDoor_C"))
  (bind _output_get (set `self.Elevator Door` _returnvalue)))

(event `self.Box.OnComponentBeginOverlap`
  (params (OverlappedComponent :type "PrimitiveComponent Object Reference") (OtherActor :type "Actor Object Reference") (OtherComp :type "PrimitiveComponent Object Reference") (OtherBodyIndex :type Integer) (bFromSweep :type Boolean) (SweepResult :type "HitResult Structure (by ref)"))
  (if (`self.Valid`)
    (`self.K2_SetActorLocation` (stale `self.ReceiveBeginPlay` _output_get) (+ (`SceneComponent.K2_GetComponentLocation` (`/Game/Blueprints/ElevatorDoor.StaticMesh` (`self.Elevator Door`))) (250.0 0.0 0.0)) false false)
    (set `self.Valid` false)))

(fn `UserConstructionScript`)