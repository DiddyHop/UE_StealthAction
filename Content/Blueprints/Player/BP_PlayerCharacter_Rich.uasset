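; Player character Blueprint implementing hitscan shooting with fire-rate limiting, timed reloads from an ammo pool and weapon heat.
; AttackCalled runs Gunshot, or starts a reload when the clip is empty, using timers for both delays.
; Gunshot line-traces along the actor's right vector, applies damage and spawns a pooled Niagara impact.
; Each shot adds heat that widens random spread and scales camera shake, while Tick cools it per frame and prints it.
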(event `AttackCalled`
  ;[1 0.05616 0.2263] Shooting
  (if (`self.isReloading`)
    _
    (elif (`self.canShoot`)
      (if (> (`self.CurrentClip`) 0)
        (set `self.canShoot` false)
        (`self.Gunshot`)
        (set `self.CurrentClip` (- (`self.CurrentClip`) 1))
        (`KismetSystemLibrary.K2_SetTimerDelegate` (delegate `FireRateCool`) (`self.fireRate`))
        (else
          ;[0.4158 1 0.1317] Reloading
          (set `self.isReloading` true)
          (`KismetSystemLibrary.PrintString` "Reloading..." true true (struct :`R` 1.0 :`G` 0.98969 :`A` 1.0))
          (`KismetSystemLibrary.K2_SetTimerDelegate` (delegate `Reloading`) (`self.reloadDuration`)))))))

(event `FireRateCool`
  ;[1 0.05616 0.2263] Shooting
  (set `self.canShoot` true))

(event `Reloading`
  ;[0.4158 1 0.1317] Reloading
  (if (> (`self.AmmoPool`) 30)
    (set `self.AmmoPool` (- (`self.AmmoPool`) 30))
    (set `self.CurrentClip` 30)
    (else
      (set `self.CurrentClip` (`self.AmmoPool`))
      (set `self.AmmoPool` 0)))
  (`KismetSystemLibrary.PrintString` "Reloaded!" true true (struct :`R` 0.002218 :`G` 1.0 :`A` 1.0))
  (set `self.isReloading` false))

(event `self.ReceiveTick`
  (params (DeltaSeconds :type "Float (single-precision)"))
  (if (> (`self.weaponHeat`) 0.0)
    (set `self.weaponHeat` (- (`self.weaponHeat`) (`self.heatCooldownRate`)))
    (`KismetSystemLibrary.PrintString` (`KismetStringLibrary.Conv_DoubleToString` (`self.weaponHeat`)) true true (struct :`G` 0.66 :`B` 1.0 :`A` 1.0) 1.0)
    (else
      (set `self.weaponHeat` 0.0))))

(fn `CalculateSpread`
  (params (Initial :type "Vector Structure"))
  (returns (Final :type "Vector Structure"))
  (if (`KismetMathLibrary.RandomBool`)
    (set `self.randomSpread` (+ (`KismetMathLibrary.MakeVector` Initial_X Initial_Y Initial_Z) (`KismetMathLibrary.RandomFloatInRange` 0.0 (`self.weaponHeat`))))
    (else
      (bind _output_get (set `self.randomSpread` (- (`KismetMathLibrary.MakeVector` Initial_X Initial_Y Initial_Z) (`KismetMathLibrary.RandomFloatInRange` 0.0 (`self.weaponHeat`)))))))
  (return _output_get))

(fn `Gunshot`
  (bind (_returnvalue_location _returnvalue_rotation) (`KismetMathLibrary.BreakTransform` (`self.GetTransform`)))
  (bind _outhit (`KismetSystemLibrary.LineTraceSingle` :`Start` (+ _returnvalue_location (0.0 0.0 50.0)) :`End` (`self.CalculateSpread` (+ _returnvalue_location (* (`KismetMathLibrary.GetRightVector` _returnvalue_rotation) (`self.shootRange`)))) :`TraceChannel` "TraceTypeQuery1" :`DrawDebugType` "ForDuration" :`DrawTime` 1.0))
  (bind (_bblockinghit _binitialoverlap _time _distance _location _impactpoint _normal _impactnormal _physmat _hitactor) (`GameplayStatics.BreakHitResult` _outhit))
  (`self.ImpactFX` 0 _location (`KismetMathLibrary.Conv_VectorToRotator` _impactnormal))
  (`GameplayStatics.ApplyDamage` _hitactor (`self.shotDamage`))
  (set `self.weaponHeat` (+ (`self.weaponHeat`) (`self.heatPerShot`)))
  (`LegacyCameraShake.StartLegacyCameraShake` null null (`self.weaponHeat`)))

(fn `ImpactFX`
  (params (Material :type Integer) (Location :type "Vector Structure") (Rotation :type "Rotator Structure"))
  (`NiagaraFunctionLibrary.SpawnSystemAtLocation` "/Game/Blueprints/FX/NS_BulletImpact.NS_BulletImpact" Location Rotation (1.0 1.0 1.0) false true "AutoRelease"))

(fn `UserConstructionScript`)