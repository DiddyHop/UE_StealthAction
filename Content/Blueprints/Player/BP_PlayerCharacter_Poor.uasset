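; BP_PlayerCharacter_Poor is a player character variant that starts without a gun and shows its own HUD.
; On BeginPlay it clears HasGun, then creates the WB_HUD_Poor widget and adds it to the viewport.
; AttackCalled runs Attack only when CanAttack is set, then clears that flag and starts a cooldown timer that re-enables attacking.
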(event `self.ReceiveBeginPlay`
  (set `self.hasGun` false)
  (bind _returnvalue (`|CreateWidget` "/Game/UI/WB_HUD_Poor.WB_HUD_Poor_C"))
  (`UserWidget.AddToViewport` _returnvalue 0))

(event `self.AttackCalled`
  (if (`self.canAttack`)
    (`self.Attack`)
    (set `self.canAttack` false)
    (`KismetSystemLibrary.K2_SetTimerDelegate` (delegate `PrepareAttack`) (`self.attackCooldown`))))

(event `PrepareAttack`
  (set `self.canAttack` true))

(fn `UserConstructionScript`
  (`parent.UserConstructionScript`))