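; BP_AI is an AI character Blueprint that exposes helper functions for patrol and movement.
; It returns its stored patrol route and maps an Idle, Walking or Sprinting state to the CharacterMovement max walk speed, returning the value set.
; A teardown function destroys both the capsule component and an attached spotlight.
; The file holds no decision logic or events, and its construction script is empty.
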(fn `DestroyCapsule`
  (`ActorComponent.K2_DestroyComponent` (`self.CapsuleComponent`))
  (`ActorComponent.K2_DestroyComponent` (`self.SpotLight`)))

(fn `GetPatrolRoute`
  (returns (PatrolRoute :type "/Game/Blueprints/AI/BP_spline Object Reference"))
  (return (`self.PatrolRoute`)))

(fn `SetMovementSpeed`
  (params (Speed :type "/Game/Blueprints/AI/enums/E_MovementSpeed Enum" :default "NewEnumerator0"))
  (returns (SpeedValue :type "Float (double-precision)"))
  (bind _output_get (set `CharacterMovementComponent.MaxWalkSpeed` (select `/Game/Blueprints/AI/enums/E_MovementSpeed` Speed :`NewEnumerator1` 200.0 :`NewEnumerator2` 500.0 :!type "Float (single-precision)") (`self.CharacterMovement`)))
  (return _output_get))

(fn `UserConstructionScript`)